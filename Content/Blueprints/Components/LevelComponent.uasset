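; Actor component that tracks a Unit's experience and level and supplies level-based stat bonuses.
; A lazy one-time init builds a level map from the level table in the unit's data table row, applies initial levels, then fully restores HP/MP.
; AddExp accumulates experience and recursively levels up while thresholds are met.
; GetAddParam returns the current level's value for the requested stat, while GetMulParam is always neutral.
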(event Custom|AddExp
  (params (AddExp :type Float%20%28single-precision%29))
  ;[1 1 1] AddExp
  (Utilities|CheckInit
    (:Inited
      (Variables|Default|SetExp (+ AddExp (Variables|Default|GetExp)))
      (CallFunction|LevelUp))))

(event EventBeginPlay)

(event EventTick
  (params (DeltaSeconds :type Float%20%28single-precision%29)))

(fn Init
  (Utilities|Map|Clear (Variables|Default|GetUnitLevelData))
  (Variables|Default|SetLv 0)
  (bind _asunit (Utilities|Casting|CastToUnit (Components|GetOwner)))
  (bind _returnvalue (Utilities|GetDataTableRow "/Game/DataTables/UnitDataTable.UnitDataTable" (Variables|/Game/Blueprints/Units/Unit.Unit_C|GetUnitKey _asunit))
    (:then
      (bind _outrownames (DataTable|GetDataTableRowNames (.LevelDataTable (Utilities|Struct|BreakUnitData _returnvalue))))
      (for _array_element _outrownames
        (bind _returnvalue_2 (Utilities|GetDataTableRow (.LevelDataTable (Utilities|Struct|BreakUnitData _returnvalue)) _array_element)
          (:then
            (Utilities|Map|Add (Variables|Default|GetUnitLevelData) (Math|Conversions|ToInteger(Byte) (Utilities|String|ToString(Name) _array_element)) _returnvalue_2))))
      (CallFunction|LevelUp)
      (Default|FullRecovery (Actor|GetComponentbyClass (Components|GetOwner) "/Game/Blueprints/Components/HPMPComponent.HPMPComponent_C")))))

(fn LevelUp
  (bind _unitleveldata (Variables|Default|GetUnitLevelData))
  (bind _lv (Variables|Default|GetLv))
  (bind _returnvalue (+ _lv 1))
  (bind (_value _returnvalue_2) (Utilities|Map|Find _unitleveldata _returnvalue))
  (if _returnvalue_2
    (if (>= (Variables|Default|GetExp) (.Exp (Utilities|Struct|BreakUnitLevelData _value)))
      (Math|Integer|IncrementInt (Variables|Default|GetLv)
        (:%20%20
          (CallFunction|LevelUp))))))

(fn GetAddParam
  (params (Param :type Param%20Enum :default "NewEnumerator0"))
  (bind _lv (Variables|Default|GetLv))
  (bind _unitleveldata (Variables|Default|GetUnitLevelData))
  (bind _value (Utilities|Map|Find _unitleveldata _lv))
  (bind (_exp _hp _mp _hpregen _mpregen _meleeattack _magicpower _defence _magicresist _attackspeed _attackrange _movementspeed) (Utilities|Struct|BreakUnitLevelData _value))
  (Utilities|CheckInit
    (:Inited
      (return (Utilities|Select :Index Param :NewEnumerator0 _hp :NewEnumerator1 _mp :NewEnumerator2 _hpregen :NewEnumerator3 _mpregen :NewEnumerator4 _meleeattack :NewEnumerator5 _magicpower :NewEnumerator6 _defence :NewEnumerator7 _magicresist :NewEnumerator8 _attackspeed :NewEnumerator10 _attackrange :NewEnumerator9 _movementspeed)))))

(fn GetMulParam
  (params (Param :type Param%20Enum :default "NewEnumerator0"))
  (Utilities|CheckInit
    (:Inited
      (return 1.0))))