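; Actor component that tracks current HP and MP for its owning Unit, with an alive check based on HP.
; Maximums are not stored here; macros cast the owner to Unit and query its parameters, halting if the cast fails.
; AddHP and AddMP apply changes clamped between zero and those maximums.
; FullRecovery sets both values to maximum, while PercentRecovery feeds a fraction of each maximum through the clamped add events.
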(event Custom|PercentRecovery
  (params (Percent :type Float%20%28single-precision%29))
  ;[1 1 1] PercentRecovery
  (bind _maxhp (Utilities|GetMaxHP)
    (:Get
      (CallFunction|AddHP (* _maxhp Percent))
      (bind _value (Utilities|GetMaxMP)
        (:Get
          (CallFunction|AddMP (* _value Percent)))))))

(event Custom|AddMP
  (params (Amount :type Float%20%28single-precision%29))
  ;[1 1 1] AddMP
  (bind _value (Utilities|GetMaxMP)
    (:Get
      (Variables|Default|SetCurMP (Math|Float|Clamp(Float) (+ Amount (Variables|Default|GetCurMP)) 0.0 _value)))))

(event Custom|FullRecovery
  ;[1 1 1] FullRecovery
  (bind _maxhp (Utilities|GetMaxHP)
    (:Get
      (Variables|Default|SetCurHP _maxhp)
      (bind _value (Utilities|GetMaxMP)
        (:Get
          (Variables|Default|SetCurMP _value))))))

(event Custom|AddHP
  (params (Amount :type Float%20%28single-precision%29))
  ;[1 1 1] AddHP
  (bind _maxhp (Utilities|GetMaxHP)
    (:Get
      (Variables|Default|SetCurHP (Math|Float|Clamp(Float) (+ Amount (Variables|Default|GetCurHP)) 0.0 _maxhp)))))

(event EventBeginPlay)

(event EventTick
  (params (DeltaSeconds :type Float%20%28single-precision%29)))

(fn IsAlive
  (return (> (Variables|Default|GetCurHP) 0.0)))