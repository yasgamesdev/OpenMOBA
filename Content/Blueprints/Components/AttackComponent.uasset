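; Unit attack component that runs server-side combat against the TargetComponent's target while the micro command is Attack.
; Each Tick refreshes timings and ranges from unit parameters and data table rates, then drives a timed Ready, Attacking, Cooldown state machine.
; A separate hold range governs continued attacks; leaving it triggers an AI chase, after cooldown if cooling down.
; Attacks stop and face the unit, then apply damage and dispatch an event.
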(event Custom|Attack
  (params (Actor :type Actor%20Object%20Reference))
  ;[1 1 1] Attack
  (bind _asunit (Utilities|Casting|CastToUnit (Components|GetOwner)))
  (bind _owner (Default|GetOwnerUnit _asunit))
  (bind _value (Default|GetUnitParam _asunit "NewEnumerator4"))
  (Class|AISenseDamage|ReportDamageEvent Actor _owner _value "0, 0, 0")
  (Game|Damage|ApplyDamage Actor _value 0 _owner)
  (Default|DispatchNormalEvent _asunit "NewEnumerator2"))

(event EventBeginPlay)

(event EventTick
  (params (DeltaSeconds :type Float%20%28single-precision%29))
  (bind _returnvalue (Components|GetOwner))
  ;[1 1 1] Tick
  (if (Ability|HasAuthority _returnvalue)
    (CallFunction|SetAttackParam)
    (bind _asunit (Utilities|Casting|CastToUnit _returnvalue))
    (switch Utilities|FlowControl|Switch|SwitchonMicroCommand (Variables|/Game/Blueprints/Units/Unit.Unit_C|GetMicroCommand _asunit)
      (:NewEnumerator0
        (switch Utilities|FlowControl|Switch|SwitchonAttackState (Variables|Default|GetAttackState) :!label _label
          (:NewEnumerator1
            (Variables|Default|SetAttackState "NewEnumerator0")
            (Variables|Default|SetTimer 0.0))
          (:NewEnumerator2
            (bind _output_get (Variables|Default|SetTimer (+ (Variables|Default|GetTimer) (Utilities|Time|GetWorldDeltaSeconds))))
            (if (>= _output_get (Variables|Default|GetCooldownTime))
              (Variables|Default|SetAttackState "NewEnumerator0")
              (Variables|Default|SetTimer 0.0)))))
      (:NewEnumerator1
        (goto _label))
      (:NewEnumerator2
        (Utilities|IsValid (Variables|Default|GetTargetUnit)
          (:Is%20Valid
            (bind _asunit_2 (Utilities|Casting|CastToUnit (Components|GetOwner)))
            (bind _distance (CallFunction|GetUnitDistance _asunit_2 (Variables|Default|GetTargetUnit)))
            (switch Utilities|FlowControl|Switch|SwitchonAttackState (Variables|Default|GetAttackState)
              (:NewEnumerator0
                (if (<= _distance (Variables|Default|GetAttackStartRange))
                  (Utilities|StopMovement
                    (:Stop
                      (Utilities|SetOwnerAnimState "NewEnumerator2"
                        (:Set
                          (Utilities|SetOwnerRotation (Variables|Default|GetTargetUnit)
                            (:Set
                              (Variables|Default|SetAttackState "NewEnumerator1")
                              (bind _output_get_2 (Variables|Default|SetTimer (+ (Variables|Default|GetTimer) (Utilities|Time|GetWorldDeltaSeconds))))
                              (if (>= _output_get_2 (Variables|Default|GetAttackingTime))
                                (CallFunction|Attack (Variables|Default|GetTargetUnit))
                                (Variables|Default|SetAttackState "NewEnumerator2")
                                (Variables|Default|SetTimer 0.0))))))))))
              (:NewEnumerator1
                (if (<= _distance (Variables|Default|GetAttackHoldRange))
                  (Utilities|StopMovement
                    (:Stop
                      (Utilities|SetOwnerAnimState "NewEnumerator2"
                        (:Set
                          (Utilities|SetOwnerRotation (Variables|Default|GetTargetUnit)
                            (:Set
                              (bind _output_get_3 (Variables|Default|SetTimer (+ (Variables|Default|GetTimer) (Utilities|Time|GetWorldDeltaSeconds))))
                              (if (>= _output_get_3 (Variables|Default|GetAttackingTime))
                                (CallFunction|Attack (Variables|Default|GetTargetUnit))
                                (Variables|Default|SetAttackState "NewEnumerator2")
                                (Variables|Default|SetTimer 0.0))))))))
                  (else
                    (Utilities|SetOwnerAnimState "NewEnumerator1"
                      (:Set
                        (Variables|Default|SetAttackState "NewEnumerator0")
                        (Variables|Default|SetTimer 0.0)
                        (AI|AIMoveTo (AI|GetAIController (Components|GetOwner)) "0, 0, 0" (Variables|Default|GetTargetUnit) -1.0 "Default" "Default" true true))))))
              (:NewEnumerator2
                (if (<= _distance (Variables|Default|GetAttackHoldRange))
                  (bind _output_get_4 (Variables|Default|SetTimer (+ (Variables|Default|GetTimer) (Utilities|Time|GetWorldDeltaSeconds))))
                  (if (>= _output_get_4 (Variables|Default|GetCooldownTime))
                    (Variables|Default|SetAttackState "NewEnumerator1")
                    (Variables|Default|SetTimer 0.0))
                  (else
                    (bind _output_get_5 (Variables|Default|SetTimer (+ (Variables|Default|GetTimer) (Utilities|Time|GetWorldDeltaSeconds))))
                    (if (>= _output_get_5 (Variables|Default|GetCooldownTime))
                      (Utilities|SetOwnerAnimState "NewEnumerator1"
                        (:Set
                          (Variables|Default|SetAttackState "NewEnumerator0")
                          (Variables|Default|SetTimer 0.0)
                          (AI|AIMoveTo (AI|GetAIController (Components|GetOwner)) "0, 0, 0" (Variables|Default|GetTargetUnit) -1.0 "Default" "Default" true true)))))))))
          (:Is%20Not%20Valid
            (goto _label)))))))

(fn SetAttackParam
  (bind _returnvalue (Components|GetOwner))
  (bind _asunit (Utilities|Casting|CastToUnit _returnvalue))
  (bind _returnvalue_2 (Utilities|GetDataTableRow "/Game/DataTables/UnitDataTable.UnitDataTable" (Variables|/Game/Blueprints/Units/Unit.Unit_C|GetUnitKey _asunit))
    (:then
      (Utilities|FlowControl|Sequence
        (:then_0
          (bind _value (Default|GetUnitParam _asunit "NewEnumerator8"))
          (Variables|Default|SetAttackingTime (* _value (.PreliminaryActionRate (Utilities|Struct|BreakUnitData _returnvalue_2))))
          (Variables|Default|SetCooldownTime (* _value (- 1.0 (.PreliminaryActionRate (Utilities|Struct|BreakUnitData _returnvalue_2))))))
        (:then_1
          (bind _value_2 (Default|GetUnitParam _asunit "NewEnumerator10"))
          (Variables|Default|SetAttackStartRange _value_2)
          (Variables|Default|SetAttackHoldRange (* _value_2 (.AttackHoldRangeRate (Utilities|Struct|BreakUnitData _returnvalue_2)))))
        (:then_2
          (bind _unit (Default|GetTargetUnit (Actor|GetComponentbyClass _returnvalue "/Game/Blueprints/Components/TargetComponent.TargetComponent_C")))
          (Variables|Default|SetTargetUnit _unit))))))